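; BP_ObjectSpawner is an actor that scatters copies of a mesh through a spherical volume around itself.
; The construction script adds SpawnCount local-space instances to an InstancedStaticMesh component, each in a random direction within SpawnRadius with random rotation and uniform scale.
; Because distance is drawn linearly, instances cluster toward the center, and the event graph has no runtime logic.
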(event `self.ReceiveBeginPlay`)

(fn `UserConstructionScript`
  (bind _returnvalue (`KismetMathLibrary.RandomFloatInRange` 0.0 360.0))
  (for _ (range (`self.SpawnCount`))
    (`InstancedStaticMeshComponent.AddInstance` (`self.InstancedStaticMesh`) (`KismetMathLibrary.MakeTransform` (* (`KismetMathLibrary.RandomUnitVector`) (`KismetMathLibrary.RandomFloatInRange` 0.0 (`self.SpawnRadius`))) (`KismetMathLibrary.MakeRotator` _returnvalue _returnvalue _returnvalue) (`KismetMathLibrary.Conv_DoubleToVector` (`KismetMathLibrary.RandomFloatInRange` 0.5 2.0))) false)))